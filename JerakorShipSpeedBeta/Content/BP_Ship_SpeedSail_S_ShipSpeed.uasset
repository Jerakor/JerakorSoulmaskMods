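; Speed sail ship part that drives a cosmetic trail effect while attached to a space raft character.
; Each tick, the trail turns on only while the sail is extended and active, with width and line alpha scaled by the parent raft's velocity and clamped.
; A RunNetMode macro limits trail updates to standalone, client and listen server, and the emitter is destroyed at BeginPlay on dedicated servers.
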(event EventBeginPlay
  (|CallParentFunction)
  (Utilities|RunNetMode
    (:DedicatedServer
      (Components|DestroyComponent (Variables|Default|GetTrailEffectEmitter)))))

(event Collision|EventActorBeginOverlap
  (params (OtherActor :type Actor%20Object%20Reference))
  (|CallParentFunction OtherActor) ; This node is disabled and will not be called.\nDrag off pins to build functionality.
)

(event EventTick
  (params (DeltaSeconds :type Float%20%28single-precision%29))
  (|CallParentFunction DeltaSeconds)
  (CallFunction|UpdateTrailEffectTick))

(fn ConstructionScript
  (|CallParentFunction))

(fn UpdateTrailEffectTick
  (bind _traileffectemitter (Variables|Default|GetTrailEffectEmitter))
  (bind _traileffectemitter_2 (Variables|Default|GetTrailEffectEmitter))
  (bind _traileffectemitter_3 (Variables|Default|GetTrailEffectEmitter))
  (bind _traileffectcolor (Variables|RefitWing|GetTrailEffectColor))
  (bind (_r _g _b) (Utilities|Struct|BreakLinearColor _traileffectcolor))
  (bind _returnvalue (Components|Activation|IsActive _traileffectemitter_3))
  (Utilities|RunNetMode
    (:Standalone
      _)
    (:NetClient
      _)
    (:ListenServer
      _))
  (if (Utilities|Enum|Equal(Enum) (Variables|Default|GetCurrentAnimState) "RRWAState_Extended")
    (Utilities|FlowControl|Sequence
      (:then_0
        (if (Variables|Default|GetbIsActived)
          (if (not _returnvalue)
            (Components|Activation|Activate _traileffectemitter_3 false))
          (elif _returnvalue
            (Components|Activation|Deactivate _traileffectemitter_3))))
      (:then_2
        (if (Variables|Default|GetbIsActived)
          (bind _ashcharacter_raft_space (Utilities|Casting|CastToHCharacterRaftSpace (Actor|GetAttachParentActor)))
          (Effects|Components|ParticleSystem|SetFloatParameter _traileffectemitter_2 "Width" (Math|Float|Clamp(Float) (Math|Float|Square (/ (Math|Vector|VectorLength (Variables|/Script/Engine.MovementComponent|GetVelocity (Variables|/Script/Engine.Character|GetCharacterMovement _ashcharacter_raft_space))) 5e+02)) 0.5 1e+01))
          (Niagara|SetNiagaraVariable(LinearColor) _traileffectemitter_2 "LineColor" (Utilities|Struct|MakeLinearColor _r _g _b (Math|Float|Clamp(Float) (/ (Math|Vector|VectorLength (Variables|/Script/Engine.MovementComponent|GetVelocity (Variables|/Script/Engine.Character|GetCharacterMovement _ashcharacter_raft_space))) 1.2e+03) 0.3 1.5))))))
    (elif (Components|Activation|IsActive _traileffectemitter)
      (Components|Activation|Deactivate _traileffectemitter))))